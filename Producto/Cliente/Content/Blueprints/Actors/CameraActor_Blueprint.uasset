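; Finish-line camera Blueprint for the racing game that takes over from the player when the race ends and shows the classification screen.
; Tick polls the player-finished flag on the level object held by BP_RaceGameInstance.
; Once it is set, a one-shot Created guard adds WBP_Classification to the viewport, shows the mouse cursor and has the player controller possess this Blueprint.
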(event `self.ReceiveBeginPlay`)

(event `self.ReceiveTick`
  (params (DeltaSeconds :type "Float (single-precision)"))
  (bind _returnvalue (`GameplayStatics.GetPlayerController` 0))
  (bind _asbp_race_game_instance (cast `/Game/Blueprints/GameModes/BP_RaceGameInstance` (`GameplayStatics.GetGameInstance`)))
  (if (`RacingLevel.GetPlayerHasFinished` (`RaceGameInstance.GetLevel` _asbp_race_game_instance))
    (if (not (`self.created`))
      (bind _returnvalue_2 (`|CreateWidget` "/Game/Blueprints/UI/WBP_Classification.WBP_Classification_C"))
      (`UserWidget.AddToViewport` _returnvalue_2 0)
      (set `PlayerController.bShowMouseCursor` true _returnvalue)
      (`Controller.Possess` _returnvalue self)
      (set `self.created` true))))

(fn `UserConstructionScript`)