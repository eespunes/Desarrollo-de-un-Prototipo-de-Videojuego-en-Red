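; Race start lights actor that plays the countdown for the first player's vehicle and releases it to race.
; While the pawn's race component allows a start, Tick uses a timer-based Wait macro to light red LEDs one by one with a sound.
; After the last, it turns them green by swapping mesh materials and sets CanRace.
; When starting is no longer allowed, green LEDs go black and the sequence resets.
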(event `self.ReceiveTick`
  (params (DeltaSeconds :type "Float (single-precision)"))
  (bind _asvehicle_pawn (cast `VehiclePawn` (`GameplayStatics.GetPlayerPawn` 0)))
  (bind _returnvalue (`VehiclePawn.GetRaceComponent` _asvehicle_pawn))
  (if (`RaceComponent.CanStartRace` _returnvalue)
    (if (`self.sequencePlayed`)
      _
      (elif (== (`self.Current Light`) 4)
        (`self.Wait` 1.0 DeltaSeconds)
        (for (_array_element _array_index) (`MeshComponent.GetMaterials` (`self.StaticMeshComponent`))
          (if (== _array_element "/Game/Assets/Materials/Automotive/Emissive/MI_LED_Red.MI_LED_Red")
            (`PrimitiveComponent.SetMaterial` (`self.StaticMeshComponent`) _array_index "/Game/Assets/Materials/Automotive/Emissive/MI_LED_Green.MI_LED_Green")))
        (`RaceComponent.SetCanRace` _returnvalue true)
        (set `self.sequencePlayed` true)
        (else
          (`self.Wait` 1.0 DeltaSeconds)
          (`PrimitiveComponent.SetMaterial` (`self.StaticMeshComponent`) (+ (`self.Current Light`) 2) "/Game/Assets/Materials/Automotive/Emissive/MI_LED_Red.MI_LED_Red")
          (`GameplayStatics.PlaySound2D` "/Game/Assets/Audio/Starting_light_sound.Starting_light_sound" 1.0 1.0 0.0 null null)
          (`/Engine/EditorBlueprintResources/StandardMacros.IncrementInt` (`self.Current Light`)))))
    (else
      (for (_array_element_2 _array_index_2) (`MeshComponent.GetMaterials` (`self.StaticMeshComponent`))
        (if (== _array_element_2 "/Game/Assets/Materials/Automotive/Emissive/MI_LED_Green.MI_LED_Green")
          (`PrimitiveComponent.SetMaterial` (`self.StaticMeshComponent`) _array_index_2 "/Game/Assets/Materials/Automotive/Emissive/MI_LED_Black.MI_LED_Black")))
      (set `self.sequencePlayed` false)
      (set `self.Current Light` 0))))

(fn `UserConstructionScript`)